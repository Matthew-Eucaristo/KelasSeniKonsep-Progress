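; Ada Wong character Blueprint exposing montage-driven action events for punching, kicking, shooting, insulting, reacting to hits and dying.
; Punch (also on debug key X) and Martelo kick wait a fraction of the montage length, then share one pass damaging overlapping Characters in HitArea.
; Hit reaction disables input until its montage ends, death quits the game afterward, and shooting and insulting only play animations.
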(event Custom|Dies
  (bind _returnvalue (Animation|PlayAnimMontage "/Game/Characters/AdaWong/Dying_Montage.Dying_Montage" 1.0 "None"))
  (Utilities|FlowControl|Delay _returnvalue)
  (Game|QuitGame 0 "Quit" false))

(event Custom|Insult
  (Animation|PlayAnimMontage "/Game/Characters/AdaWong/Insult_Montage.Insult_Montage" 1.0 "None"))

(event Custom|Martelo%20Kick
  (bind _returnvalue (Animation|PlayAnimMontage "/Game/Characters/AdaWong/Martelo_2_Montage.Martelo_2_Montage" 1.0 "None"))
  (Utilities|FlowControl|Delay (/ _returnvalue 2.35))
  (for _array_element (Collision|GetOverlappingActors (Variables|Default|GetHit%20Area) "/Script/Engine.Character" :!class /Script/Engine.PrimitiveComponent)
    (Game|Damage|ApplyDamage _array_element 1e+02 0 0)
    (Development|PrintString "Hello")))

(event Custom|Punch
  (bind _returnvalue (Animation|PlayAnimMontage "/Game/Characters/AdaWong/Punching_Montage.Punching_Montage" 1.0 "None"))
  (Utilities|FlowControl|Delay (* _returnvalue 0.333333))
  (for _array_element (Collision|GetOverlappingActors (Variables|Default|GetHit%20Area) "/Script/Engine.Character" :!class /Script/Engine.PrimitiveComponent)
    (Game|Damage|ApplyDamage _array_element 1e+02 0 0)
    (Development|PrintString "Hello")))

(event Custom|Get%20Reaction%20Hit
  (Input|DisableInput 0)
  (bind _returnvalue (Animation|PlayAnimMontage "/Game/Characters/AdaWong/Reaction_Montage.Reaction_Montage" 1.0 "None"))
  (Utilities|FlowControl|Delay _returnvalue)
  (Input|EnableInput 0))

(event Custom|Shoot
  (Animation|PlayAnimMontage "/Game/Characters/AdaWong/Shooting_Montage.Shooting_Montage" 1.0 "None"))

(event EventBeginPlay)

(event Collision|EventActorBeginOverlap
  (params (OtherActor :type Actor%20Object%20Reference)))

(event Input|KeyboardEvents|DebugKeyX
  (params (Key :type Key%20Structure :default "None") (ActionValue :type Input%20Action%20Value%20Structure))
  (:Pressed
    (bind _returnvalue (Animation|PlayAnimMontage "/Game/Characters/AdaWong/Punching_Montage.Punching_Montage" 1.0 "None"))
    (Utilities|FlowControl|Delay (* _returnvalue 0.333333))
    (for _array_element (Collision|GetOverlappingActors (Variables|Default|GetHit%20Area) "/Script/Engine.Character" :!class /Script/Engine.PrimitiveComponent)
      (Game|Damage|ApplyDamage _array_element 1e+02 0 0)
      (Development|PrintString "Hello"))))

(fn ConstructionScript)